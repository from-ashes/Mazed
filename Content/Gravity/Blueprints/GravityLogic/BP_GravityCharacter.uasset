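; Gravity character Blueprint that handles level-start setup on top of its parent class.
; BeginPlay silences its audio, then a timeline drives the volume multiplier.
; The timeline's first update also sets game-only input, sets LevelComplete0 true and switches on EdgeEffectToggle in the WorldCollection material parameter collection.
; The first capsule hit sets LevelComplete0 back to false, guarded by a DoOnce.
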(event `self.ReceiveBeginPlay`
  (bind _audio_0 (`self.Audio_0`))
  (`AudioComponent.SetVolumeMultiplier` _audio_0 0.0)
  (bind (_direction _newtrack_0) (`Timeline|Timeline_0_0` :!via `PlayFromStart`)
    (:`Update`
      (`AudioComponent.SetVolumeMultiplier` _audio_0 _newtrack_0)
      (`/Engine/EditorBlueprintResources/StandardMacros.DoOnce` false
        (:`Completed`
          (`WidgetBlueprintLibrary.SetInputMode_GameOnly` (`GameplayStatics.GetPlayerController` 0))
          (set `self.LevelComplete_0` true)
          (`KismetMaterialLibrary.SetScalarParameterValue` "/Game/Assets/WorldCollection.WorldCollection" "EdgeEffectToggle" 1.0))))))

(event `self.CapsuleComponent.OnComponentHit`
  (params (HitComponent :type "PrimitiveComponent Object Reference") (OtherActor :type "Actor Object Reference") (OtherComp :type "PrimitiveComponent Object Reference") (NormalImpulse :type "Vector Structure") (Hit :type "HitResult Structure (by ref)"))
  (`/Engine/EditorBlueprintResources/StandardMacros.DoOnce` false
    (:`Completed`
      (set `self.LevelComplete_0` false))))

(fn `UserConstructionScript`
  (`parent.UserConstructionScript`))